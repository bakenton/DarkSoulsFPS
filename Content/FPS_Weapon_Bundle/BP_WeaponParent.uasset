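; BP_WeaponParent is a weapon Blueprint, named as a parent class, that handles firing through its Shooting event.
; When IsShooting is true, it spawns BP_Bullet at FireArrow, plays a gunshot sound, attaches an explosion emitter and briefly reveals a PointLight as muzzle flash.
; It also adds a camera shake source component per shot and runs a forward line trace whose result is unused.
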(event EventShooting
  (params (bIsShooting? :type Boolean))
  (bind _firearrow (Variables|Default|GetFireArrow))
  (bind _firearrow_2 (Variables|Default|GetFireArrow))
  (bind _returnvalue (Transformation|GetWorldLocation _firearrow))
  (bind _returnvalue_2 (Transformation|GetWorldTransform _firearrow_2))
  (if bIsShooting?
    (Game|SpawnActorfromClass "/Game/FPS_Weapon_Bundle/BP_Bullet.BP_Bullet_C" (Math|Transform|MakeTransform (.location _returnvalue_2) (.rotation _returnvalue_2) "1.000000,1.000000,1.000000") "Undefined" "MultiplyWithRoot" 0 0)
    (Development|SetHiddeninGame (Variables|Default|GetPointLight) false false)
    (Audio|SpawnSound2D "/Game/Map/Music/SC_GunShoot.SC_GunShoot" 1.0 1.0 0.0 0)
    (Collision|LineTraceByChannel _returnvalue (+ _returnvalue (* (Math|Vector|GetForwardVector (Transformation|GetWorldRotation _firearrow)) 3e+03)) "TraceTypeQuery1" false 0 "None")
    (AddComponent|AddCameraShakeSourceComponent false)
    (Effects|SpawnEmitterAttached "/Game/StarterContent/Particles/P_Explosion.P_Explosion" (Variables|Default|GetFireArrow) "None" "0, 0, 0" "0, 0, 0" "0.100000,0.100000,0.100000" "SnapToTargetIncludingScale")
    (Utilities|FlowControl|Delay 0.1)
    (Development|SetHiddeninGame (Variables|Default|GetPointLight) true false)))

(fn ConstructionScript)