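; Bullet actor that plays surface-specific impact effects when it hits something, then destroys itself.
; On Hit, a visibility sphere trace runs from the hit location, using the raw hit normal as its end point, to read the physical material.
; The surface type selects the sound and particle emitter spawned at the trace's hit location, with variants for concrete, wood and a default.
; It contains no damage logic.
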(event Collision|EventHit
  (params (MyComp :type Primitive%20Component%20Object%20Reference) (Other :type Actor%20Object%20Reference) (OtherComp :type Primitive%20Component%20Object%20Reference) (bSelfMoved :type Boolean) (HitLocation :type Vector :default "0, 0, 0") (HitNormal :type Vector :default "0, 0, 0") (NormalImpulse :type Vector :default "0, 0, 0") (Hit :type Hit%20Result%20Structure%20%28by%20ref%29))
  (Utilities|IsValid self
    (:Is%20Valid
      _)
    (:Is%20Not%20Valid
      _))
  (bind _outhit (Collision|SphereTraceByChannel HitLocation HitNormal 0.0 "TraceTypeQuery1" false 0 "None"))
  (Audio|SpawnSoundatLocation (Utilities|Select :Index (Variables|/Script/PhysicsCore.PhysicalMaterial|GetSurfaceType (.PhysMat (Collision|BreakHitResult _outhit))) :SurfaceType_Default "/Game/Free_UI/CUE/Abstract1_Cue.Abstract1_Cue" :SurfaceType1 "/Game/SmallSoundKit/SSKCue/FootstepsCue/S_Concrete_Mono_1_Cue.S_Concrete_Mono_1_Cue" :SurfaceType2 "/Game/SmallSoundKit/SSKCue/FootstepsCue/S_Wood_Mono_1_Cue.S_Wood_Mono_1_Cue") (.Location (Collision|BreakHitResult _outhit)) "0, 0, 0" 1.0 1.0 0.0 0 0)
  (Effects|SpawnEmitteratLocation (Utilities|Select :Index (Variables|/Script/PhysicsCore.PhysicalMaterial|GetSurfaceType (.PhysMat (Collision|BreakHitResult _outhit))) :SurfaceType_Default "/Game/StarterContent/Particles/P_Ambient_Dust.P_Ambient_Dust" :SurfaceType1 "/Game/Realistic_Starter_VFX_Pack_Vol2/Particles/Hit/P_Concrete.P_Concrete" :SurfaceType2 "/Game/Realistic_Starter_VFX_Pack_Vol2/Particles/Destruction/P_Destruction_Wood.P_Destruction_Wood") (.Location (Collision|BreakHitResult _outhit)))
  (Actor|DestroyActor))

(fn ConstructionScript)